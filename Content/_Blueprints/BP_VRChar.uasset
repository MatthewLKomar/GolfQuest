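; VR player character for a golf game, with a club and a toggleable menu widget.
; On BeginPlay it picks the tracking origin from the HMD device name, using floor level for Oculus and SteamVR and eye level with a raised VR root for PSVR.
; Club hits on a BP_Ball increment the global stroke count in BP_GolfState, and the MenuToggle input switches the menu's visibility.
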(event OnComponentHit(Club)
  (params (HitComponent :type Primitive%20Component%20Object%20Reference) (OtherActor :type Actor%20Object%20Reference) (OtherComp :type Primitive%20Component%20Object%20Reference) (NormalImpulse :type Vector :default "0, 0, 0") (Hit :type Hit%20Result%20Structure%20%28by%20ref%29))
  (Utilities|Casting|CastToBP_Ball OtherActor)
  (bind _asbp_golf_state (Utilities|Casting|CastToBP_GolfState (Game|GetGameState)))
  (Variables|/Game/_Blueprints/BP_GolfState.BP_GolfState_C|SetstrikesGlobal _asbp_golf_state (+ (Variables|/Game/_Blueprints/BP_GolfState.BP_GolfState_C|GetstrikesGlobal _asbp_golf_state) 1)))

(event EventBeginPlay
  (switch name (Class|HeadMountedDisplayFunctionLibrary|GetHMDDeviceName) ; TODO: Add one for WMR
    (:OculusHMD
      (Class|HeadMountedDisplayFunctionLibrary|SetTrackingOrigin "Floor" :!label _label) ; Windows (Vive/Oculus)
    )
    (:SteamVR
      (goto _label))
    (:PSVR
      (Class|HeadMountedDisplayFunctionLibrary|SetTrackingOrigin "Eye") ; PS4
      (Transformation|AddLocalOffset (Variables|Default|GetVRRoot) (Math|Vector|MakeVector 0.0 0.0 91.0) false false))))

(event Input|ActionEvents|InputActionMenuToggle
  (params (Key :type Key%20Structure :default "None"))
  (bind _menu (Variables|Default|GetMenu))
  (bind _returnvalue (UserInterface|GetWidget _menu))
  (:Pressed
    (Widget|SetVisibility _returnvalue (Utilities|Select :Index (Widget|GetVisibility _returnvalue) :Visible "Hidden" :Collapsed "Visible" :Hidden "Visible" :HitTestInvisible "Visible" :SelfHitTestInvisible "Visible"))))

(fn ConstructionScript)