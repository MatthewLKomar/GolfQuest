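; Level positioning actor that places the alpha course and ball within the player's VR Guardian play area.
; On BeginPlay it reads the Guardian play-area boundary points and takes the midpoint of the first and fourth as the center.
; It then spawns BP_AlphaCourse at that center and BP_Ball slightly above it.
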(event EventBeginPlay
  (CallFunction|SetPlayAreaVariables)
  (Game|SpawnActorfromClass "/Game/_Blueprints/BP_AlphaCourse.BP_AlphaCourse_C" (Math|Transform|MakeTransform (Variables|Default|GetPlayAreaCenter) "0, 0, 0" "1,1,1") "Undefined" 0 0)
  (Game|SpawnActorfromClass "/Game/_Blueprints/BP_Ball.BP_Ball_C" (Math|Transform|MakeTransform (+ (Variables|Default|GetPlayAreaCenter) "0.000000, 0,50.000000") "0, 0, 0" "1,1,1") "Undefined" 0 0))

(event Collision|EventActorBeginOverlap
  (params (OtherActor :type Actor%20Object%20Reference)))

(event EventTick
  (params (DeltaSeconds :type Float%20%28single-precision%29)))

(fn ConstructionScript)

(fn SetPlayAreaVariables
  (Variables|Default|SetPlayAreaPoints (Class|OculusFunctionLibrary|GetGuardianPoints "Boundary_PlayArea" false))
  (Variables|Default|SetPlayArea0 (Utilities|Array|Get(acopy) (Variables|Default|GetPlayAreaPoints)))
  (Variables|Default|SetPlayArea1 (Utilities|Array|Get(acopy) (Variables|Default|GetPlayAreaPoints) 3))
  (Variables|Default|SetPlayAreaCenter (+ (/ (- (Utilities|Array|Get(acopy) (Variables|Default|GetPlayAreaPoints) 3) (Utilities|Array|Get(acopy) (Variables|Default|GetPlayAreaPoints))) 2.0) (Utilities|Array|Get(acopy) (Variables|Default|GetPlayAreaPoints)))))