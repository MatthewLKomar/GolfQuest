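; Procedural generator child Blueprint that fits its generation bounds to the player's VR Guardian play area at runtime.
; On BeginPlay it converts the play-area dimensions to map units via MapUnitScaler, truncating X and Y and fixing Z in BoundVector.
; It then moves and rotates the actor to the play-area transform before calling the parent BeginPlay, so inherited logic runs with the updated bounds and placement.
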(event EventBeginPlay
  (CallFunction|SetBoundVectortoPlayArea)
  (CallFunction|ApplyPlayAreaTransformation)
  (|CallParentFunction))

(event Collision|EventActorBeginOverlap
  (params (OtherActor :type Actor%20Object%20Reference)))

(event EventTick
  (params (DeltaSeconds :type Float%20%28single-precision%29)))

(fn ConstructionScript
  (|CallParentFunction))

(fn SetBoundVectortoPlayArea
  (bind _returnvalue (Class|OculusFunctionLibrary|GetGuardianDimensions "Boundary_PlayArea"))
  (bind _mapunitscaler (Variables|Default|GetMapUnitScaler))
  (bind _returnvalue_2 (/ _returnvalue _mapunitscaler))
  (Variables|Default|SetBoundVector (Utilities|Struct|MakeIntVector (Math|Float|Truncate (.x _returnvalue_2)) (Math|Float|Truncate (.y _returnvalue_2)) 3)))

(fn ApplyPlayAreaTransformation
  (bind _returnvalue (Class|OculusFunctionLibrary|GetPlayAreaTransform))
  (Transformation|SetActorLocationAndRotation (.location _returnvalue) (.rotation _returnvalue)))