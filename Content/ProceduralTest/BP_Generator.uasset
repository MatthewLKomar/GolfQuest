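; Procedural generator that builds a seeded random ball-and-hole course from tile meshes on a bounded grid.
; A looping timer advances a random walk one free horizontal neighbor at a time, storing each cell's connections as direction bitmasks.
; Bitmasks select data table rows for each tile's mesh and transform.
; At the length limit or a dead end, it caps the path and spawns the ball and hole trigger; debug inputs clear, rebuild or reseed.
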(event Custom|EVENT_StepGeneration
  (bind _mapunitscaler (Variables|MapBuild|GetMapUnitScaler))
  (bind _playgrid (Variables|InternalGeneration|GetPlayGrid))
  (bind _prospectivecollection (Variables|MapBuild|GetProspectiveCollection))
  ;[1 1 1] Stepwise Generation
  (Utilities|FlowControl|Gate false :!label _label
    (:Exit
      (bind (_previousvalue _newlocations) (InternalGeneration|StepWiseGeneration (Variables|MapBuild|GetProspectiveLocation) (Variables|InternalGeneration|GetPlayGrid) (Variables|InternalGeneration|GetRandomGenerator) (Variables|InternalGeneration|GetcustomInitialPosition)))
      (if (and (> _previousvalue 0) (< (Variables|MapBuild|GetTracking) (Variables|InternalGeneration|GetLengthParameter)))
        (Variables|MapBuild|SetTracking (+ (Variables|MapBuild|GetTracking) 1))
        (for _array_element _newlocations ; Preempt subsequent node placement
          (Utilities|Array|Add (Variables|MapBuild|GetProspectiveCollection) (CallFunction|IntVectorAdd (Variables|MapBuild|GetProspectiveLocation) (CallFunction|DirectionalVectorfromIndex _array_element)))
          (CallFunction|3DArraySet (Variables|InternalGeneration|GetPlayGrid) (CallFunction|IntVectorAdd (Variables|MapBuild|GetProspectiveLocation) (CallFunction|DirectionalVectorfromIndex _array_element)) (InternalGeneration|ConvertNodeValues (.Forward (CallFunction|DirectionsfromIndex (Utilities|Select :Index _array_element :Option%200 1 :Option%201 0 :Option%202 3 :Option%203 2))) (.Back (CallFunction|DirectionsfromIndex (Utilities|Select :Index _array_element :Option%200 1 :Option%201 0 :Option%202 3 :Option%203 2))) (.Left (CallFunction|DirectionsfromIndex (Utilities|Select :Index _array_element :Option%200 1 :Option%201 0 :Option%202 3 :Option%203 2))) (.Right (CallFunction|DirectionsfromIndex (Utilities|Select :Index _array_element :Option%200 1 :Option%201 0 :Option%202 3 :Option%203 2))) (.Up (CallFunction|DirectionsfromIndex (Utilities|Select :Index _array_element :Option%200 1 :Option%201 0 :Option%202 3 :Option%203 2))) (.Down (CallFunction|DirectionsfromIndex (Utilities|Select :Index _array_element :Option%200 1 :Option%201 0 :Option%202 3 :Option%203 2)))))
          (Development|PrintString (Utilities|String|Append (Utilities|String|ToString(Integer) (InternalGeneration|ConvertNodeValues (.Forward (CallFunction|DirectionsfromIndex (Utilities|Select :Index _array_element :Option%200 1 :Option%201 0 :Option%202 3 :Option%203 2))) (.Back (CallFunction|DirectionsfromIndex (Utilities|Select :Index _array_element :Option%200 1 :Option%201 0 :Option%202 3 :Option%203 2))) (.Left (CallFunction|DirectionsfromIndex (Utilities|Select :Index _array_element :Option%200 1 :Option%201 0 :Option%202 3 :Option%203 2))) (.Right (CallFunction|DirectionsfromIndex (Utilities|Select :Index _array_element :Option%200 1 :Option%201 0 :Option%202 3 :Option%203 2))) (.Up (CallFunction|DirectionsfromIndex (Utilities|Select :Index _array_element :Option%200 1 :Option%201 0 :Option%202 3 :Option%203 2))) (.Down (CallFunction|DirectionsfromIndex (Utilities|Select :Index _array_element :Option%200 1 :Option%201 0 :Option%202 3 :Option%203 2))))) " at " (Utilities|String|ToString(Integer) (CallFunction|IntVectorAdd (Variables|MapBuild|GetProspectiveLocation) (CallFunction|DirectionalVectorfromIndex _array_element)))) true true "(R=1.000000,G=0.000000,B=0.470354,A=1.000000)"))
        ;;[1 0.6652 0.9916] Finalize placement step on current branch
        (CallFunction|3DArraySet _playgrid (Variables|MapBuild|GetProspectiveLocation) (Class|KismetMathLibrary|OrIntInt (CallFunction|3DArrayGet _playgrid (Variables|MapBuild|GetProspectiveLocation)) _previousvalue))
        (Utilities|PlaceMesh (Math|Color|Lerp(LinearColor) "(R=0.651945,G=0.000000,B=1.000000,A=1.000000)" "(R=0.039463,G=1.000000,B=0.000000,A=1.000000)" (/ (Math|Conversions|ToFloat(Integer) (Variables|MapBuild|GetTracking)) (Math|Conversions|ToFloat(Integer) (Variables|InternalGeneration|GetLengthParameter)))) (Variables|MapBuild|GetProspectiveLocation) (CallFunction|3DArrayGet _playgrid (Variables|MapBuild|GetProspectiveLocation)))
        ;;[1 1 1] Prepare next node to check
        (Variables|MapBuild|SetProspectiveLocation (Utilities|Array|Get(acopy) _prospectivecollection))
        (Utilities|Array|RemoveIndex _prospectivecollection)
        (else
          (Development|PrintString "EndPoint Trapped!" true true "(R=1.000000,G=0.005761,B=0.000000,A=1.000000)" 5.0)
          (Rendering|Debug|DrawDebugBox :Center (* (Math|Conversions|ToVector(Float) (Variables|MapBuild|GetProspectiveLocation)) _mapunitscaler) :Extent (Math|Conversions|ToVector(Float) _mapunitscaler))
          (Utilities|PlaceMesh "(R=0.000000,G=0.841327,B=1.000000,A=1.000000)" (Variables|MapBuild|GetProspectiveLocation) -2)
          (MapBuild|SpawnBallandHole)
          (Utilities|Time|ClearandInvalidateTimerbyHandle (Variables|MapBuild|GetTimingStructure))
          (goto _label Close))))))

(event Custom|EVENT_InitializeGeneration
  (CallFunction|EVENTClearMap)
  (if (not (Utilities|Time|IsValidTimerHandle (Variables|MapBuild|GetTimingStructure)))
    (bind _returnvalue (Utilities|Time|SetTimerbyEvent (delegate Custom|EVENT_StepGeneration) (* 0.25 (/ 1.0 (Variables|Default|GetAnimationRate))) true))
    (Variables|MapBuild|SetTimingStructure _returnvalue)))

(event Custom|EVENT_ClearMap
  (bind _meshes (Variables|MapBuild|GetMeshes))
  (bind _mapunitscaler (Variables|MapBuild|GetMapUnitScaler))
  (bind _playgrid (Variables|InternalGeneration|GetPlayGrid))
  (bind _prospectivecollection (Variables|MapBuild|GetProspectiveCollection))
  ;[1 1 1] Clear Map
  (Utilities|Time|ClearandInvalidateTimerbyHandle (Variables|MapBuild|GetTimingStructure))
  (Variables|MapBuild|SetTracking 0)
  (bind _outactors (Actor|GetAllActorsOfClass "/Game/_Blueprints/BP_Ball.BP_Ball_C"))
  (for _array_element _outactors
    (Actor|DestroyActor _array_element))
  (bind _outactors_2 (Actor|GetAllActorsOfClass "/Game/_Blueprints/BP_HoleTrigger.BP_HoleTrigger_C"))
  (for _array_element_2 _outactors_2
    (Actor|DestroyActor _array_element_2))
  (for _array_element_3 _meshes
    (Components|DestroyComponent _array_element_3))
  (Utilities|Array|Clear _meshes)
  (Development|PrintString "Destroyed Map!")
  (MapBuild|PrimeMap)
  ;[1 1 1] Stepwise Generation
  (Utilities|FlowControl|Gate false) ; enters at Open
)

(event EventBeginPlay
  ;[1 1 1] Begin Play: Generate Initial Tile and subsequent tile info: Tobe Macro
  (Components|Timeline|SetPlayRate (Variables|Default|GetMeshAnimatingTimeline) (Variables|Default|GetAnimationRate))
  (Variables|InternalGeneration|SetRandomGenerator (Math|Random|MakeRandomStream (Variables|InternalGeneration|GetInitial%20Seed)))
  (MapBuild|PrimeMap))

(event Input|ActionEvents|InputActionBPress
  (params (Key :type Key%20Structure :default "None"))
  ;[1 1 1] Clear Map
  (:Pressed
    (CallFunction|EVENTClearMap)))

(event Input|ActionEvents|InputActionAPress
  (params (Key :type Key%20Structure :default "None"))
  (:Pressed
    (if (not (Utilities|Time|IsValidTimerHandle (Variables|MapBuild|GetTimingStructure)))
      (bind _returnvalue (Utilities|Time|SetTimerbyEvent (delegate Custom|EVENT_StepGeneration) (* 0.25 (/ 1.0 (Variables|Default|GetAnimationRate))) true))
      (Variables|MapBuild|SetTimingStructure _returnvalue))))

(event Input|KeyboardEvents|B
  (params (Key :type Key%20Structure :default "None"))
  (:Pressed
    (if (not (Utilities|Time|IsValidTimerHandle (Variables|MapBuild|GetTimingStructure)))
      (bind _returnvalue (Utilities|Time|SetTimerbyEvent (delegate Custom|EVENT_StepGeneration) (* 0.25 (/ 1.0 (Variables|Default|GetAnimationRate))) true))
      (Variables|MapBuild|SetTimingStructure _returnvalue))))

(event Input|KeyboardEvents|0
  (params (Key :type Key%20Structure :default "None"))
  ;[1 1 1] Increment Random Seed
  (:Pressed
    (bind _output_get (Variables|InternalGeneration|SetInitial%20Seed (+ (Variables|InternalGeneration|GetInitial%20Seed) 1)))
    (Development|PrintString (Utilities|String|ToString(Integer) _output_get) true true "(R=1.000000,G=1.000000,B=1.000000,A=1.000000)")
    (Variables|InternalGeneration|SetRandomGenerator (Math|Random|MakeRandomStream (Variables|InternalGeneration|GetInitial%20Seed)))))

(event Input|KeyboardEvents|N
  (params (Key :type Key%20Structure :default "None"))
  ;[1 1 1] Clear Map
  (:Pressed
    (CallFunction|EVENTClearMap)))

(fn ConstructionScript
  (bind _box (Variables|Default|GetBox))
  (bind _mapunitscaler (Variables|MapBuild|GetMapUnitScaler))
  (bind _boundvector (Variables|InternalGeneration|GetBoundVector))
  (bind _returnvalue (/ 2.0 _mapunitscaler))
  (bind _returnvalue_2 (Math|Conversions|ToVector(Float) _boundvector))
  (bind _returnvalue_3 (/ _returnvalue_2 _returnvalue))
  (Components|Box|SetBoxExtent _box _returnvalue_3 false)
  (Transformation|SetWorldLocation _box (+ (Transformation|GetWorldLocation (Variables|Default|GetDefaultSceneRoot)) _returnvalue_3) false false))

(fn MakeNodeGrid
  (params (NewSize :type Int%20Vector%20Structure))
  (bind (_x _y _z) (Utilities|Struct|BreakIntVector NewSize))
  (Utilities|Array|Resize (LocalVariables|GetnewArray) (* _x _y _z))
  (return (Utilities|Struct|MakeF_3DArray (LocalVariables|GetnewArray) NewSize)))

(fn SelectStartingNode
  (params (Dimensions :type Int%20Vector%20Structure))
  (bind (_x _y _z) (Utilities|Struct|BreakIntVector Dimensions))
  (return (select (Variables|InternalGeneration|GetuseCustomInitalPosition) (Variables|InternalGeneration|GetcustomInitialPosition) (Utilities|Struct|MakeIntVector 0 (/ _y 2) (/ _z 2)))))

(fn ConvertNodeValues
  (params (Foward :type Boolean) (Back :type Boolean) (Left :type Boolean) (Right :type Boolean) (Up :type Boolean) (Down :type Boolean))
  (return (+ (Math|Integer|SelectInt 1 0 Foward) (Math|Integer|SelectInt 2 0 Back) (Math|Integer|SelectInt 4 0 Left) (Math|Integer|SelectInt 8 0 Right) (Math|Integer|SelectInt 16 0 Up) (Math|Integer|SelectInt 32 0 Down))))

(fn UnConvertNodeValues
  (params (NodeValue :type Integer))
  (return (Utilities|Struct|MakeF_DirectionTracker (> (Class|KismetMathLibrary|AndIntInt NodeValue 1) 0) (> (Class|KismetMathLibrary|AndIntInt NodeValue 2) 0) (> (Class|KismetMathLibrary|AndIntInt NodeValue 4) 0) (> (Class|KismetMathLibrary|AndIntInt NodeValue 8) 0) (> (Class|KismetMathLibrary|AndIntInt NodeValue 16) 0) (> (Class|KismetMathLibrary|AndIntInt NodeValue 32) 0))))

(fn CheckNodeOccupancy
  (params (Nodes :type F%203D%20Array%20Structure) (Location :type Int%20Vector%20Structure))
  (return (== (CallFunction|3DArrayGet Nodes Location) 0)))

(fn CheckNodeinBounds
  (params (BoundsVector :type Int%20Vector%20Structure%20%28by%20ref%29) (TestVector :type Int%20Vector%20Structure%20%28by%20ref%29))
  (bind (_x _y _z) (Utilities|Struct|BreakIntVector BoundsVector))
  (bind (_x_2 _y_2 _z_2) (Utilities|Struct|BreakIntVector TestVector))
  (return (Math|Boolean|ANDBoolean (< _x_2 _x) (< _y_2 _y) (< _z_2 _z) (>= _x_2 0) (>= _y_2 0) (>= _z_2 0))))

(fn StepWiseGeneration
  (params (Previous%20Step :type Int%20Vector%20Structure) (CurrentGrid :type F%203D%20Array%20Structure%20%28by%20ref%29) (StreamToUse :type Random%20Stream%20Structure%20%28by%20ref%29) (ReferencePosition :type Int%20Vector%20Structure))
  (bind _selecteddirections (LocalVariables|GetSelectedDirections))
  (bind _output (Utilities|Array|Get(acopy) _selecteddirections))
  (bind (_forward _back _left _right _up _down) (CallFunction|DirectionsfromIndex _output))
  (LocalVariables|SetTempLocation Previous%20Step)
  (bind _output_get (LocalVariables|SetProspectiveLocations (Utilities|Array|MakeArray (CallFunction|IntVectorAdd (CallFunction|DirectionalVectorfromIndex) (LocalVariables|GetTempLocation)) (CallFunction|IntVectorAdd (CallFunction|DirectionalVectorfromIndex 1) (LocalVariables|GetTempLocation)) (CallFunction|IntVectorAdd (CallFunction|DirectionalVectorfromIndex 2) (LocalVariables|GetTempLocation)) (CallFunction|IntVectorAdd (CallFunction|DirectionalVectorfromIndex 3) (LocalVariables|GetTempLocation)))))
  (Utilities|Array|Clear (LocalVariables|GetNextDirections))
  (for (_array_element _array_index) _output_get
    (if (and (InternalGeneration|CheckNodeinBounds (.Size (Utilities|Struct|BreakF_3DArray CurrentGrid)) _array_element) (InternalGeneration|CheckNodeOccupancy CurrentGrid _array_element))
      (Utilities|Array|Add (LocalVariables|GetNextDirections) _array_index)))
  (if (> (Utilities|Array|Length (LocalVariables|GetNextDirections)) 0)
    (Utilities|Array|Add (LocalVariables|GetSelectedDirections) (.OutItem (Utilities|Array|RandomFromStream (LocalVariables|GetNextDirections) StreamToUse)))
    (LocalVariables|SetLastNodeValue (InternalGeneration|ConvertNodeValues _forward _back _left _right _up _down))
    (for _array_element_2 (LocalVariables|GetSelectedDirections)
      (Utilities|Array|Add (LocalVariables|GetSelectedLocations) _array_element_2))
    (return (LocalVariables|GetLastNodeValue) (LocalVariables|GetSelectedLocations))
    (else
      (return 0 0))))

(fn MeshPlacementFunction
  (params (Value :type Linear%20Color%20Structure) (InIntVector :type Int%20Vector%20Structure%20%28by%20ref%29) (Selection :type Integer))
  (Utilities|FlowControl|Sequence
    (:then_0
      (if (< Selection 0)
        (Utilities|FlowControl|Sequence
          (:then_0
            (switch int Selection ; Default places  decorative components
              (:-2
                (LocalVariables|SetAssetRowName "End")
                (LocalVariables|SetSelfRotation 9e+01))
              (:-1
                (LocalVariables|SetAssetRowName "Begin"))))
          (:then_1
            (bind _desireddirection (CallFunction|IndexfromDirections (InternalGeneration|UnConvertNodeValues (CallFunction|3DArrayGet (Variables|InternalGeneration|GetPlayGrid) InIntVector))))
            (Development|PrintString (Utilities|String|ToString(Integer) _desireddirection) true true "(R=1.000000,G=0.442140,B=0.314001,A=1.000000)" 5.0)
            (LocalVariables|SetSelfRotation (+ (LocalVariables|GetSelfRotation) (Utilities|Select :Index _desireddirection :Option%200 0.0 :Option%201 1.8e+02 :Option%202 2.7e+02 :Option%203 9e+01)))
            (LocalVariables|SetMeshTransform (Math|Transform|MakeTransform "0, 0, 0" (Math|Rotator|MakeRotator 0.0 0.0 (LocalVariables|GetSelfRotation))))))
        (else
          ;[1 1 1] Common Tiles all defined as positive directions
          (LocalVariables|SetAssetRowName (Utilities|String|StringToName (Utilities|String|ToString(Integer) Selection))))))
    (:then_1
      (bind _returnvalue (Utilities|GetDataTableRow (Variables|MapBuild|GetData%20Table) (LocalVariables|GetAssetRowName))
        (:then
          (LocalVariables|SetMeshClass (.AssetClass (Utilities|Struct|BreakF_AssetTableRow _returnvalue)))
          (LocalVariables|SetMeshTransform (Math|Transform|ComposeTransforms (.Transform (Utilities|Struct|BreakF_AssetTableRow _returnvalue)) (LocalVariables|GetMeshTransform))))
        (:RowNotFound
          (Development|PrintString "Where da Asset At?")
          (return 0 ""))))
    (:then_2
      (bind _returnvalue_2 (AddComponent|AddStaticMeshComponent true))
      (Utilities|Array|Add (Variables|MapBuild|GetMeshes) _returnvalue_2)
      (Components|StaticMesh|SetStaticMesh _returnvalue_2 (LocalVariables|GetMeshClass))
      (return _returnvalue_2 (Math|Transform|ComposeTransforms (LocalVariables|GetMeshTransform) (Math|Transform|MakeTransform (* (Math|Conversions|ToVector(Float) InIntVector) (Variables|MapBuild|GetMapUnitScaler))))))))

(fn PrimeMap
  (bind _boundvector (Variables|InternalGeneration|GetBoundVector))
  (bind (_x _y _z) (Utilities|Struct|BreakIntVector _boundvector))
  (bind _gridpoints (InternalGeneration|MakeNodeGrid (Utilities|Struct|MakeIntVector _x _y _z)))
  (bind _output_get (Variables|InternalGeneration|SetPlayGrid _gridpoints))
  (bind _startingnode (InternalGeneration|SelectStartingNode (.Size (Utilities|Struct|BreakF_3DArray _output_get))))
  (Variables|InternalGeneration|SetcustomInitialPosition _startingnode)
  (CallFunction|3DArraySet (Variables|InternalGeneration|GetPlayGrid) (Variables|InternalGeneration|GetcustomInitialPosition) (InternalGeneration|ConvertNodeValues true false false false false false))
  (Utilities|PlaceMesh "(R=1.000000,G=0.000000,B=0.000000,A=1.000000)" (Variables|InternalGeneration|GetcustomInitialPosition) -1)
  (bind _output_get_2 (Variables|MapBuild|SetProspectiveLocation (CallFunction|IntVectorAdd (Variables|InternalGeneration|GetcustomInitialPosition) (CallFunction|DirectionalVectorfromIndex))))
  (CallFunction|3DArraySet (Variables|InternalGeneration|GetPlayGrid) _output_get_2 (InternalGeneration|ConvertNodeValues false true false false false false)))

(fn SpawnBallandHole
  (bind _meshes (Variables|MapBuild|GetMeshes))
  (bind _returnvalue (Utilities|Array|Length _meshes))
  (bind _returnvalue_2 (- _returnvalue 1))
  (bind _output (Utilities|Array|Get(acopy) _meshes _returnvalue_2))
  (bind _returnvalue_3 (Transformation|GetWorldLocation _output))
  ;[1 1 1] Spawn a ball at the course start (i.e. the position of the 0th tile)
  (Game|SpawnActorfromClass "/Game/_Blueprints/BP_Ball.BP_Ball_C" (Math|Transform|MakeTransform (+ (Transformation|GetWorldLocation (Utilities|Array|Get(acopy) (Variables|MapBuild|GetMeshes))) "0, 0,50.000000")) "Undefined" 0 0)
  ;[1 1 1] Spawn a hole trigger at the course end (i.e. the position of the (n-1)th tile)
  (Game|SpawnActorfromClass "/Game/_Blueprints/BP_HoleTrigger.BP_HoleTrigger_C" (Math|Transform|MakeTransform (Math|Vector|MakeVector (.x _returnvalue_3) (.y _returnvalue_3) (- (.z (Transformation|GetWorldLocation (Utilities|Array|Get(acopy) _meshes))) 25.0))) "Undefined" 0 0))